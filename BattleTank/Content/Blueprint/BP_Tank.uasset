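; BP_Tank is a player-driven tank pawn with movement and orbit-camera aiming from axis inputs.
; Aim input yaws AzimuthGimbal and pitches SpringArm at delta-time-scaled speeds, with optional elevation inversion; BeginPlay sets the arm's roll inheritance.
; Forward input adds movement along the actor's facing, while Turn adds raw axis value to actor yaw each frame, unscaled by delta time.
; Strafing logic exists but is disconnected.
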(event EventBeginPlay
  (Variables|/Script/Engine.SpringArmComponent|SetbInheritRoll (Variables|Default|GetSpringArm) (Variables|Default|GetInheritRoll)))

(event Input|AxisEvents|InputAxisAimAzimuth
  (params (AxisValue :type Float%20%28single-precision%29))
  ;[1 1 1] Camera Input Binding
  (Transformation|AddLocalRotation (Variables|Default|GetAzimuthGimbal) (Math|Rotator|MakeRotator 0.0 0.0 (* AxisValue (Utilities|Time|GetWorldDeltaSeconds) (Variables|Default|GetAzimuthSpeed))) false false))

(event Input|AxisEvents|InputAxisAimElevation
  (params (AxisValue :type Float%20%28single-precision%29))
  (bind _returnvalue (Utilities|Time|GetWorldDeltaSeconds))
  (bind _elevationspeed (Variables|Default|GetElevationSpeed))
  (bind _returnvalue_2 (* AxisValue _returnvalue _elevationspeed))
  ;[1 1 1] Camera Input Binding
  (if (Variables|Default|GetInvertElevation)
    (Transformation|AddLocalRotation (Variables|Default|GetSpringArm) (Math|Rotator|MakeRotator 0.0 (* _returnvalue_2 -1.0) 0.0) false false)
    (else
      (Transformation|AddLocalRotation (Variables|Default|GetSpringArm) (Math|Rotator|MakeRotator 0.0 _returnvalue_2 0.0) false false))))

(event Input|AxisEvents|InputAxisTurn
  (params (AxisValue :type Float%20%28single-precision%29))
  (bind _returnvalue (Transformation|GetActorRotation))
  (bind (_roll _pitch _yaw) (Math|Rotator|BreakRotator _returnvalue))
  (Transformation|SetActorRotation (Math|Rotator|MakeRotator _roll _pitch (+ AxisValue _yaw))))

(event Input|AxisEvents|InputAxisForward
  (params (AxisValue :type Float%20%28single-precision%29))
  (Pawn|Input|AddMovementInput (Math|Vector|GetForwardVector (Transformation|GetActorRotation)) AxisValue true))

(fn ConstructionScript)